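; RTS camera pawn that pans, zooms and rotates over the map.
; Enhanced Input from IMC_RTS drives planar movement, clamped spring-arm zoom and a held rotate action that turns mouse X delta into yaw.
; Tick adds edge scrolling when the cursor nears a viewport border, one direction at a time, then clamps the pawn's X and Y to a fixed square boundary.
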(event Input|EnhancedActionEvents|EnhancedInputActionIA_CameraZoom
  (params (ActionValue :type Float%20%28double-precision%29) (ElapsedSeconds :type Float%20%28double-precision%29) (TriggeredSeconds :type Float%20%28double-precision%29) (InputAction :type Input%20Action%20Object%20Reference :default "/Game/Aetherforge/Input/IA_CameraZoom.IA_CameraZoom"))
  (Variables|/Script/Engine.SpringArmComponent|SetTargetArmLength (Variables|Default|GetSpringArm) (Math|Float|Clamp(Float) (+ (* ActionValue (Variables|Default|GetZoomSpeed)) (Variables|/Script/Engine.SpringArmComponent|GetTargetArmLength (Variables|Default|GetSpringArm))) 3e+02 2e+03)))

(event Input|EnhancedActionEvents|EnhancedInputActionIA_CameraRotate
  (params (ActionValue :type Boolean) (ElapsedSeconds :type Float%20%28double-precision%29) (TriggeredSeconds :type Float%20%28double-precision%29) (InputAction :type Input%20Action%20Object%20Reference :default "/Game/Aetherforge/Input/IA_CameraRotate.IA_CameraRotate"))
  (:Started
    (Variables|Default|SetIsRotating true))
  (:Completed
    (Variables|Default|SetIsRotating false)))

(event Input|EnhancedActionEvents|EnhancedInputActionIA_CameraMove
  (params (ActionValue :type Vector%202D%20Structure) (ElapsedSeconds :type Float%20%28double-precision%29) (TriggeredSeconds :type Float%20%28double-precision%29) (InputAction :type Input%20Action%20Object%20Reference :default "/Game/Aetherforge/Input/IA_CameraMove.IA_CameraMove"))
  (bind (_x _y) (Math|Vector2D|BreakVector2D ActionValue))
  (bind _returnvalue (Utilities|Time|GetWorldDeltaSeconds))
  (bind _panspeed (Variables|Default|GetPanSpeed))
  (Transformation|AddActorWorldOffset (+ (* (* (* _x (Transformation|GetActorRightVector)) _panspeed) _returnvalue) (* _returnvalue (* _panspeed (* _y (Transformation|GetActorForwardVector)))))))

(event EventBeginPlay
  (Input|AddMappingContext (PlayerController|LocalPlayerSubsystems|GetEnhancedInputLocalPlayerSubsystem (Game|GetPlayerController 0)) "/Game/Aetherforge/Input/IMC_RTS.IMC_RTS" 0 "(bIgnoreAllPressedKeysUntilRelease=True,bForceImmediately=False,bNotifyUserSettings=False)"))

(event EventTick
  (params (DeltaSeconds :type Float%20%28single-precision%29))
  (bind _returnvalue (Transformation|GetActorLocation))
  (bind (_x _y _z) (Math|Vector|BreakVector _returnvalue))
  (CallFunction|EdgeScroll)
  (CallFunction|MiddleMouseButtonRotate)
  (Transformation|SetActorLocation (Math|Vector|MakeVector (Math|Conversions|ToFloat(Integer) (Math|Integer|Clamp(Integer) (Math|Float|Truncate _x) -5000 5000)) (Math|Conversions|ToFloat(Integer) (Math|Integer|Clamp(Integer) (Math|Float|Truncate _y) -5000 5000)) _z) false false))

(fn ConstructionScript)

(fn EdgeScroll
  (bind _returnvalue (Game|GetPlayerController 0))
  (bind _returnvalue_2 (Game|GetPlayerController 0))
  (bind _locationy (Game|Player|GetMousePosition _returnvalue))
  (bind _locationx (Game|Player|GetMousePosition _returnvalue_2))
  ;[0.15 0.15 0.15 0.5] Edge Scroll
  (Variables|Default|SetEdgeDelta "0, 0, 0")
  (if (< _locationx (Variables|Default|GetEdgeThredshold))
    (Variables|Default|SetEdgeDelta (* (Utilities|Time|GetWorldDeltaSeconds) (* (Math|Vector|NegateVector (Transformation|GetActorRightVector)) (Variables|Default|GetEdgeSpeed))))
    (elif (> _locationx (- (.x (Viewport|GetViewportSize)) (Variables|Default|GetEdgeThredshold)))
      (Variables|Default|SetEdgeDelta (* (* (Transformation|GetActorRightVector) (Variables|Default|GetEdgeSpeed)) (Utilities|Time|GetWorldDeltaSeconds)))
      (elif (< _locationy (Variables|Default|GetEdgeThredshold))
        (Variables|Default|SetEdgeDelta (* (* (Transformation|GetActorForwardVector) (Variables|Default|GetEdgeSpeed)) (Utilities|Time|GetWorldDeltaSeconds)))
        (elif (> _locationy (- (.y (Viewport|GetViewportSize)) (Variables|Default|GetEdgeThredshold)))
          (Variables|Default|SetEdgeDelta (* (* (Math|Vector|NegateVector (Transformation|GetActorForwardVector)) (Variables|Default|GetEdgeSpeed)) (Utilities|Time|GetWorldDeltaSeconds)))
          (else
            (return))))))
  (Transformation|AddActorWorldOffset (Variables|Default|GetEdgeDelta))
  (return))

(fn MiddleMouseButtonRotate
  (if (Variables|Default|GetIsRotating)
    (Transformation|SetActorRotation (Math|Rotator|MakeRotator 0.0 0.0 (+ (* (.DeltaX (Class|PlayerController|GetInputMouseDelta (Game|GetPlayerController 0))) (Variables|Default|GetRotateSpeed)) (.Yaw (Math|Rotator|BreakRotator (Transformation|GetActorRotation))))))
    (return)
    (else
      (return))))