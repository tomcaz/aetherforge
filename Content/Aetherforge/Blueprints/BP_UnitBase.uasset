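; BP_UnitBase is a unit base Blueprint that moves toward an ordered world location.
; MoveToLocation stores the target and raises a move-order flag.
; Each Tick, while the flag is set, it adds movement input straight toward the target, with no pathfinding, and clears the flag once within a fixed arrival distance.
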(event Custom|MoveToLocation
  (params (TargetLocation :type Vector))
  (Variables|Default|SetMoveTargetLocation TargetLocation)
  (Variables|Default|SetHasMoveOrder true))

(event EventBeginPlay)

(event Collision|EventActorBeginOverlap
  (params (OtherActor :type Actor%20Object%20Reference)))

(event EventTick
  (params (DeltaSeconds :type Float%20%28single-precision%29))
  (bind _returnvalue (Transformation|GetActorLocation))
  (bind _movetargetlocation (Variables|Default|GetMoveTargetLocation))
  (bind _returnvalue_2 (- _movetargetlocation _returnvalue))
  (if (Variables|Default|GetHasMoveOrder)
    (if (> (Math|Vector|VectorLength _returnvalue_2) 1e+02)
      (Pawn|Input|AddMovementInput (Math|Vector|Normalize _returnvalue_2) 1.0 false)
      (else
        (Variables|Default|SetHasMoveOrder false)))))

(fn ConstructionScript)